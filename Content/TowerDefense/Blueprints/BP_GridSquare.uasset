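; A single cell of the tower defense build grid that tracks whether building is allowed on it.
; Cursor hover over its cube notifies a referenced Blueprint, passing the cell's build location on entry.
; CheckCollisions blocks building when non-grid actors overlap the cube and allows it when nothing overlaps, swapping red and white materials to match.
; Resize scales and centers the cell from GridElementSize, leaving a small gap between cells.
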(event OnBeginCursorOver(Cube)
  (params (TouchedComponent :type Primitive%20Component%20Object%20Reference))
  (if (Utilities|IsValid (Variables|Default|GetBlueprintReference))
    (Default|HandleBeginMouseOver (Variables|Default|GetBlueprintReference) (Transformation|GetWorldLocation (Variables|Default|GetBuildLocation)))))

(event OnEndCursorOver(Cube)
  (params (TouchedComponent :type Primitive%20Component%20Object%20Reference))
  (Default|HandleEndMouseOver (Variables|Default|GetBlueprintReference)))

(event Custom|CheckCollisions
  (bind _cube (Variables|Default|GetCube))
  (bind _overlappingactors (Collision|GetOverlappingActors _cube 0 :!class /Script/Engine.PrimitiveComponent))
  ;[1 1 1] Check Collitions
  (if (> (Utilities|Array|Length _overlappingactors) 0)
    (Variables|Default|SetNothingFound true)
    (for _index (range 0 (Utilities|Array|LastIndex _overlappingactors))
      (Utilities|Casting|CastToBP_GridSquare (Utilities|Array|Get(acopy) _overlappingactors _index)
        (:CastFailed
          (CallFunction|HandleAllowBuilding false))))
    (else
      (CallFunction|HandleAllowBuilding true))))

(event Custom|CheckCollisions_Copy
  ;[1 1 1] Check Collitions past
)

(event EventBeginPlay)

(event EventActorBeginOverlap
  (params (OtherActor :type Actor%20Object%20Reference)))

(event EventTick
  (params (DeltaSeconds :type Float%20%28single-precision%29)))

(fn ConstructionScript)

(fn Resize
  (bind _gridelementsize (Variables|Default|GetGridElementSize))
  (bind _gridelementsize_2 (Variables|Default|GetGridElementSize))
  (bind _returnvalue (- _gridelementsize_2 1e+01))
  (bind _returnvalue_2 (/ _gridelementsize 2.0))
  (bind _returnvalue_3 (/ _returnvalue 1e+02))
  (bind _returnvalue_4 (/ _returnvalue_3 2.0))
  ;[1 1 1] Setting correct scale
  (Transformation|SetRelativeScale3D (Math|Vector|MakeVector _returnvalue_3 _returnvalue_3 1.0))
  (Components|Box|SetBoxExtent (Math|Vector|MakeVector _returnvalue_4 _returnvalue_4 4e+01) true)
  ;[1 1 1] Setting correct location
  (Transformation|SetRelativeLocation (Math|Vector|MakeVector _returnvalue_2 _returnvalue_2 5e+01) false)
  (Transformation|SetRelativeLocation (Math|Vector|MakeVector _returnvalue_2 _returnvalue_2 6e+01) false))

(fn HandleAllowBuilding
  (params (Allow :type Boolean :default false))
  (if Allow
    (Variables|Default|SetAllowBuilding true)
    (Rendering|Material|SetMaterial 0 "/Game/TowerDefense/Materials/White_Mat.White_Mat")
    (else
      (Variables|Default|SetAllowBuilding false)
      (Rendering|Material|SetMaterial 0 "/Game/TowerDefense/Materials/Red_Mat.Red_Mat"))))