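; Base tower actor for a tower defense game that fires rock projectiles while anything other than a projectile is inside its range.
; RangeCylinder overlaps maintain a Targets list and start a self-repeating Fire loop, paced by RateOfFire, that stops when the list empties.
; Shots spawn along the fixed ProjectileDirection component, without aiming at targets.
; The construction script sizes a grid-snapped collision box and the range cylinder from the mesh bounds, GridSize and Range.
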(event OnComponentBeginOverlap(RangeCylinder)
  (params (OtherActor :type Actor%20Object%20Reference) (OtherComp :type Primitive%20Component%20Object%20Reference) (OtherBodyIndex :type Integer) (bFromSweep :type Boolean) (SweepResult :type Hit%20Result%20Structure%20%28by%20ref%29))
  (Utilities|Casting|CastToBP_BaseProjectile OtherActor
    (:CastFailed
      (Utilities|Array|Add (Variables|Default|GetTargets) OtherActor)
      (if (not (Variables|Default|GetFiring))
        (Variables|Default|SetFiring true)
        (CallFunction|Fire)))))

(event OnComponentEndOverlap(RangeCylinder)
  (params (OtherActor :type Actor%20Object%20Reference) (OtherComp :type Primitive%20Component%20Object%20Reference) (OtherBodyIndex :type Integer))
  (Utilities|Array|RemoveItem (Variables|Default|GetTargets) OtherActor))

(event Custom|Fire
  (bind _projectiledirection (Variables|Default|GetProjectileDirection))
  (if (> (Utilities|Array|Length (Variables|Default|GetTargets)) 0)
    (Game|SpawnActorfromClass "/Game/TowerDefense/Blueprints/Projectiles/BP_RockProjectile.BP_RockProjectile_C" (Math|Transform|MakeTransform (+ (Transformation|GetWorldLocation (Variables|Default|GetProjectileSpawn)) (* (Math|Vector|GetForwardVector _projectiledirection) 1e+03)) (Transformation|GetWorldRotation _projectiledirection)) false 0)
    (if (Variables|Default|GetFiring)
      (Utilities|FlowControl|Delay (/ 1.0 (Variables|Tower|GetRateOfFire)))
      (CallFunction|Fire))
    (else
      (Variables|Default|SetFiring false))))

(event EventBeginPlay)

(event EventActorBeginOverlap
  (params (OtherActor :type Actor%20Object%20Reference)))

(event EventTick
  (params (DeltaSeconds :type Float%20%28single-precision%29)))

(fn ConstructionScript
  (bind _towermesh (Variables|Default|GetTowerMesh))
  (bind _gridsize (Variables|Tower|GetGridSize))
  (bind _gridsize_2 (Variables|Tower|GetGridSize))
  (bind _towermesh_2 (Variables|Default|GetTowerMesh))
  (bind _gridsize_3 (Variables|Tower|GetGridSize))
  (bind _gridsize_4 (Variables|Tower|GetGridSize))
  (bind _range (Variables|Tower|GetRange))
  (bind _max (Components|StaticMesh|GetLocalBounds _towermesh_2))
  (bind _max_2 (Components|StaticMesh|GetLocalBounds _towermesh))
  (bind (_x _y _z) (Math|Vector|BreakVector _max))
  (bind (_x_2 _y_2 _z_2) (Math|Vector|BreakVector _max_2))
  (bind _returnvalue (/ _z 2.0))
  (bind _returnvalue_2 (/ _z_2 2.0))
  (bind _returnvalue_3 (Math|Float|Round _returnvalue))
  (bind _returnvalue_4 (Math|Float|Round _returnvalue_2))
  (bind _returnvalue_5 (Math|Conversions|ToFloat(Integer) _returnvalue_3))
  (bind _returnvalue_6 (Math|Conversions|ToFloat(Integer) _returnvalue_4))
  ;[1 1 1] Set collision box for grid
  (Components|Box|SetBoxExtent (Math|Vector|MakeVector (* (Math|Float|Round (/ _x _gridsize_3)) _gridsize_4) (* (Math|Float|Round (/ _y _gridsize_3)) _gridsize_4) _returnvalue_5) true)
  (Transformation|SetRelativeLocation (Math|Vector|MakeVector 0.0 0.0 _returnvalue_5) false)
  ;[1 1 1] Set range cylinder mesh
  (Transformation|SetRelativeScale3D (Math|Vector|MakeVector (+ (/ (* (Math|Float|Round (/ _x_2 _gridsize_2)) _gridsize) 5e+01) _range) (+ (/ (* (Math|Float|Round (/ _y_2 _gridsize_2)) _gridsize) 5e+01) _range) (/ _returnvalue_6 5e+01)))
  (Transformation|SetRelativeLocation (Math|Vector|MakeVector 0.0 0.0 _returnvalue_6) false))